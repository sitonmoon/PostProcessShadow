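; ShadowCapture is an actor that publishes its viewpoint to ShadowMaterialParameterCollection for the shadow generator's materials.
; Both the construction script and Tick write its location as EyePos, a point along its forward vector as At, and its up vector as UpVector.
; These form look-at view inputs, refreshed every frame in play and whenever construction reruns.
; BeginPlay only prints a startup message.
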(event `self.ReceiveBeginPlay`
  (`KismetSystemLibrary.PrintString` "PostEffectCapture begin working!"))

(event `self.ReceiveTick`
  (params (DeltaSeconds :type "Float (single-precision)"))
  (bind _returnvalue (`self.K2_GetActorLocation`))
  (`KismetMaterialLibrary.SetVectorParameterValue` "/Game/ShadowGenerator/Materials/ShadowMaterialParameterCollection.ShadowMaterialParameterCollection" "EyePos" (`KismetMathLibrary.Conv_VectorToLinearColor` _returnvalue))
  (`KismetMaterialLibrary.SetVectorParameterValue` "/Game/ShadowGenerator/Materials/ShadowMaterialParameterCollection.ShadowMaterialParameterCollection" "At" (`KismetMathLibrary.Conv_VectorToLinearColor` (+ _returnvalue (`self.GetActorForwardVector`))))
  (`KismetMaterialLibrary.SetVectorParameterValue` "/Game/ShadowGenerator/Materials/ShadowMaterialParameterCollection.ShadowMaterialParameterCollection" "UpVector" (`KismetMathLibrary.Conv_VectorToLinearColor` (`self.GetActorUpVector`))))

(fn `UserConstructionScript`
  (bind _returnvalue (`self.K2_GetActorLocation`))
  (`KismetMaterialLibrary.SetVectorParameterValue` "/Game/ShadowGenerator/Materials/ShadowMaterialParameterCollection.ShadowMaterialParameterCollection" "EyePos" (`KismetMathLibrary.Conv_VectorToLinearColor` _returnvalue))
  (`KismetMaterialLibrary.SetVectorParameterValue` "/Game/ShadowGenerator/Materials/ShadowMaterialParameterCollection.ShadowMaterialParameterCollection" "At" (`KismetMathLibrary.Conv_VectorToLinearColor` (+ _returnvalue (`self.GetActorForwardVector`))))
  (`KismetMaterialLibrary.SetVectorParameterValue` "/Game/ShadowGenerator/Materials/ShadowMaterialParameterCollection.ShadowMaterialParameterCollection" "UpVector" (`KismetMathLibrary.Conv_VectorToLinearColor` (`self.GetActorUpVector`))))